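; Player spaceship sprite for an Asteroids-style shooter on the XZ plane, briefly flashing with collision off after spawning.
; Each tick it turns toward the cursor trace, moves with interpolated inertia from axis input and wraps around screen bounds.
; Fire spawns projectiles behind a DoOnce-and-Delay cooldown.
; Meteorite overlap destroys the ship, which notifies the GameMode to attempt a respawn and spawns an actor in its place.
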(event `self.ReceiveBeginPlay`
  (bind _shipsprite (`self.ShipSprite`))
  ;[1 1 1] Begin Play - Initialize
  (`PrimitiveComponent.SetCollisionEnabled` (`self.ShipSprite`) "NoCollision")
  (add `self.OnDestroyed` (delegate `OnDestroyed_Event`))
  (`self.EnableInput` (`GameplayStatics.GetPlayerController` 0))
  (bind (_direction _value) (`Timeline|FlashingTimeline`)
    (:`Update`
      (`PaperSpriteComponent.SetSpriteColor` _shipsprite (make `LinearColor` 1.0 1.0 1.0 _value)))
    (:`Finished`
      (`PrimitiveComponent.SetCollisionEnabled` _shipsprite "QueryAndPhysics"))))

(event `OnDestroyed_Event` :!signature `self.OnDestroyed`
  (params (DestroyedActor :type "Actor Object Reference"))
  ;[1 1 1] Begin Play - Initialize
  (message `/Game/Blueprints/BP_Actions_Interface.TryToSpawnPlayer` (`GameplayStatics.GetGameMode`))
  (`|SpawnActorFromClass` "/Game/Blueprints/BP_Explosion.BP_Explosion_C" (`KismetMathLibrary.Conv_VectorToTransform` (`self.K2_GetActorLocation`)) "Undefined" "OverrideRootScale" null null))

(event `self.ReceiveTick`
  (params (DeltaSeconds :type "Float (single-precision)"))
  (bind (_returnvalue_x _returnvalue_y) (`KismetMathLibrary.BreakVector` (`self.K2_GetActorLocation`)))
  (bind _returnvalue_x_2 (`KismetMathLibrary.BreakVector` (`self.K2_GetActorLocation`)))
  (bind (_returnvalue_x_3 _returnvalue_y_2 _returnvalue_z) (`KismetMathLibrary.BreakVector` (`self.K2_GetActorLocation`)))
  (bind (_returnvalue_x_4 _returnvalue_y_3 _returnvalue_z_2) (`KismetMathLibrary.BreakVector` (`self.K2_GetActorLocation`)))
  (bind _hitresult (`PlayerController.GetHitResultUnderCursorByChannel` (`GameplayStatics.GetPlayerController` 0) "TraceTypeQuery1" true))
  (bind _returnvalue (`KismetMathLibrary.MakeVector` (`self.GetInputAxisValue`) 0.0 (`self.GetInputAxisValue`)))
  (bind _returnvalue_2 (`KismetMathLibrary.Normal` (- (`KismetMathLibrary.MakeVector` (.x (`.Location` (`GameplayStatics.BreakHitResult` _hitresult))) 0.0 (.z (`.Location` (`GameplayStatics.BreakHitResult` _hitresult)))) (`self.K2_GetActorLocation`))))
  (bind _returnvalue_3 (> (`KismetMathLibrary.VSize` _returnvalue) 0.0))
  (if (`GameplayStatics.BreakHitResult` _hitresult)
    _
    (else
      _))
  (`self.K2_SetActorRotation` (`KismetMathLibrary.MakeRotator` 0.0 (* (`KismetMathLibrary.DegAcos` (`KismetMathLibrary.Dot_VectorVector` _returnvalue_2 (0.0 0.0 1.0))) (`KismetMathLibrary.SignOfFloat` (`KismetMathLibrary.Dot_VectorVector` _returnvalue_2 (-1.0 0.0 0.0))))))
  (bind _output_get (set `self.MotionVectorTemp` (`KismetMathLibrary.VInterpTo` (`self.MotionVectorTemp`) (select `bool` _returnvalue_3 :`true` (* (`KismetMathLibrary.Normal` _returnvalue) (* (`self.Speed`) (`GameplayStatics.GetWorldDeltaSeconds`)))) (`GameplayStatics.GetWorldDeltaSeconds`) (select `bool` _returnvalue_3 :`false` 1.0 :`true` 5.0 :!type "Float (single-precision)"))))
  (`self.K2_AddActorWorldOffset` _output_get)
  (`|ExecutionSequence`
    (:`then_0`
      (if (> (`KismetMathLibrary.Abs` _returnvalue_x_2) (`self.XMax`))
        (`self.K2_SetActorLocation` (`KismetMathLibrary.MakeVector` (* (`KismetMathLibrary.SignOfFloat` _returnvalue_x_2) (- (`self.XMax`) (`self.ShipTeleportOffset`)) -1.0) _returnvalue_y_2 _returnvalue_z))))
    (:`then_1`
      (if (> (`KismetMathLibrary.Abs` _returnvalue_z_2) (`self.ZMax`))
        (`self.K2_SetActorLocation` (`KismetMathLibrary.MakeVector` _returnvalue_x _returnvalue_y (* (`KismetMathLibrary.SignOfFloat` _returnvalue_z_2) (- (`self.ZMax`) (`self.ShipTeleportOffset`)) -1.0)))))
    (:`then_2`)))

(event `InputAction|FireAction`
  (params (Key :type "Key Structure"))
  (:`Pressed`
    (`/Engine/EditorBlueprintResources/StandardMacros.DoOnce` false :!label _label
      (:`Completed`
        (bind _returnvalue (`|SpawnActorFromClass` "/Game/Blueprints/BP_Projectile.BP_Projectile_C" (`KismetMathLibrary.MakeTransform` (`self.K2_GetActorLocation`) (`self.K2_GetActorRotation`)) "AlwaysSpawn" "OverrideRootScale" null null))
        (`ProjectileMovementComponent.SetVelocityInLocalSpace` (`/Game/Blueprints/BP_Projectile.ProjectileMovement` _returnvalue) (`self.ProjectileVelocity`))
        (`KismetSystemLibrary.Delay` (`self.ProjectileCoolDown`))
        (goto _label :!via `Reset`)))))

(event `self.ShipSprite.OnComponentBeginOverlap`
  (params (OverlappedComponent :type "PrimitiveComponent Object Reference") (OtherActor :type "Actor Object Reference") (OtherComp :type "PrimitiveComponent Object Reference") (OtherBodyIndex :type Integer) (bFromSweep :type Boolean) (SweepResult :type "HitResult Structure (by ref)"))
  (cast `/Game/Blueprints/BP_Meteorite` OtherActor)
  (`self.K2_DestroyActor`))

(fn `UserConstructionScript`)