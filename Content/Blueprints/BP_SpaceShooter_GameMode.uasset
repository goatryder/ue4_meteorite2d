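; Game mode for a space shooter that runs meteorite waves, lives, score and the game HUD.
; A looping timer, its interval randomized once at BeginPlay, spawns meteorite batches at randomly picked angles by rotating an offset vector around the Y axis.
; TrytoSpawnPlayer waits, deducts a life, then respawns the ship or triggers game over.
; The best score loads from a save slot at start and is rewritten at game over if matched or beaten.
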(event `SpawnMeteorite`
  (bind _spawn_points_temp (`self.Spawn_Points_Temp`))
  ;[1 1 1] Spawn Meteorite
  (set `self.Spawn_Points_Temp` (`self.Spawn_Angles`))
  (for _ (range (+ (`KismetMathLibrary.RandomIntegerInRange` 3 5) 1))
    (`KismetArrayLibrary.Array_Shuffle` _spawn_points_temp)
    (bind _returnvalue (`|SpawnActorFromClass` "/Game/Blueprints/BP_Meteorite.BP_Meteorite_C" (`KismetMathLibrary.MakeTransform` (`KismetMathLibrary.RotateAngleAxis` (`KismetMathLibrary.MakeVector` (`self.X_Max`) 0.0 (`self.Z_Max`)) (`|GetArrayItem` _spawn_points_temp (`KismetMathLibrary.RandomInteger` (`KismetArrayLibrary.Array_Length` _spawn_points_temp))) (0.0 1.0 0.0))) "Undefined" "OverrideRootScale" null null))
    (set `/Game/Blueprints/BP_Meteorite.Type` "NewEnumerator0" _returnvalue)
    (`/Game/Blueprints/BP_Meteorite.SetMeteorite` _returnvalue "NewEnumerator0")))

(event `CheckSaveGameSlot`
  ;[1 1 1] Save Game
  (bind _returnvalue (`GameplayStatics.DoesSaveGameExist` (`self.Save_Game_Name`)))
  (if _returnvalue
    (bind _returnvalue_2 (`GameplayStatics.LoadGameFromSlot` (`self.Save_Game_Name`)))
    (bind _asbp_save_game (cast `/Game/Blueprints/BP_SaveGame` _returnvalue_2))
    (bind _output_get (set `self.Save_Game_Instance_REF` _asbp_save_game))
    (`TextBlock.SetText` (`/Game/Blueprints/BP_Game_HUD.BestScoreValue` (`self.Game_HUD_REF`)) (`KismetTextLibrary.Conv_IntToText` (`/Game/Blueprints/BP_SaveGame.BestScore` _output_get)))
    (else
      (bind _returnvalue_3 (`GameplayStatics.CreateSaveGameObject` "/Game/Blueprints/BP_SaveGame.BP_SaveGame_C"))
      (bind _output_get_2 (set `self.Save_Game_Instance_REF` _returnvalue_3))
      (bind _output_get_3 (set `/Game/Blueprints/BP_SaveGame.BestScore` 0 _output_get_2))
      (`TextBlock.SetText` (`/Game/Blueprints/BP_Game_HUD.BestScoreValue` (`self.Game_HUD_REF`)) (`KismetTextLibrary.Conv_IntToText` _output_get_3))
      (`GameplayStatics.SaveGameToSlot` _output_get_2 (`self.Save_Game_Name`)))))

(event `self.ReceiveBeginPlay`
  ;[1 1 1] BeginPlay - Initialize
  (set `self.Lives` 3)
  (set `self.Score` 0)
  (set `self.Spawn_Angles` (`|MakeArray` 0.0 60.0 120.0 180.0 240.0 300.0 :!type "Float (single-precision)"))
  (`self.SpawnMeteorite`)
  (`KismetSystemLibrary.K2_SetTimer` self "SpawnMeteorite" (`KismetMathLibrary.RandomFloatInRange` (`self.SpawnMeteoriteCooldownMin`) (`self.SpawnMeteoriteCooldownMax`)) true)
  (bind _returnvalue (`|CreateWidget` "/Game/Blueprints/BP_Game_HUD.BP_Game_HUD_C"))
  (bind _output_get (set `self.Game_HUD_REF` _returnvalue))
  (`UserWidget.AddToViewport` _output_get 0)
  (`self.CheckSaveGameSlot`))

(event `/Game/Blueprints/BP_Actions_Interface.TryToSpawnPlayer`
  ;[1 1 1] Try To Spwan Player
  (`KismetSystemLibrary.Delay` (`self.SpawnPlayerDelay`))
  (bind _output_get (set `self.Lives` (- (`self.Lives`) 1)))
  (`/Game/Blueprints/BP_Game_HUD.Update Lives` (`self.Game_HUD_REF`) _output_get)
  (`/Engine/EditorBlueprintResources/StandardMacros.CompareInt` (`self.Lives`)
    (:`>`
      (`|SpawnActorFromClass` "/Game/Blueprints/BP_SpaceShip.BP_SpaceShip_C" (`KismetMathLibrary.MakeTransform` (0.0 0.0 0.0)) "AdjustIfPossibleButDontSpawnIfColliding" "OverrideRootScale" null null))
    (:`==`
      (`/Game/Blueprints/BP_Game_HUD.GameOverEvent` (`self.Game_HUD_REF`))
      (bind _returnvalue (`GameplayStatics.LoadGameFromSlot` (`self.Save_Game_Name`)))
      (bind _asbp_save_game (cast `/Game/Blueprints/BP_SaveGame` _returnvalue))
      (bind _output_get_2 (set `self.Save_Game_Instance_REF` _asbp_save_game))
      (`/Engine/EditorBlueprintResources/StandardMacros.CompareInt` (`/Game/Blueprints/BP_SaveGame.BestScore` _output_get_2) (`self.Score`)
        (:`==`
          _)
        (:`<`
          _))
      (bind _output_get_3 (set `/Game/Blueprints/BP_SaveGame.BestScore` (`self.Score`) (`self.Save_Game_Instance_REF`)))
      (`TextBlock.SetText` (`/Game/Blueprints/BP_Game_HUD.BestScoreValue` (`self.Game_HUD_REF`)) (`KismetTextLibrary.Conv_IntToText` _output_get_3))
      (`GameplayStatics.SaveGameToSlot` (`self.Save_Game_Instance_REF`) (`self.Save_Game_Name`)))))

(event `/Game/Blueprints/BP_Actions_Interface.UpdateScore`
  (params (Value :type Integer))
  ;[1 1 1] Update Score
  (set `self.Score` (+ Value (`self.Score`)))
  (`TextBlock.SetText` (`/Game/Blueprints/BP_Game_HUD.ScoreValue` (`self.Game_HUD_REF`)) (`KismetTextLibrary.Conv_IntToText` (`self.Score`))))

(fn `UserConstructionScript`)